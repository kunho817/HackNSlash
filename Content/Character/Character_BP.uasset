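; Player character for a 2D auto-shooter that moves on the X/Z plane and quits the game when its sprite registers a hit.
; Input axes nudge the actor through interpolated location updates without sweeping.
; Every Tick spawns a Magic_Bullet aimed at the average location of all Enemy actors.
; GetExp handles experience and level-ups with a growing threshold, refreshing the EXP widget created at BeginPlay.
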(event OnComponentHit(PaperSprite)
  (params (HitComponent :type Primitive%20Component%20Object%20Reference) (OtherActor :type Actor%20Object%20Reference) (OtherComp :type Primitive%20Component%20Object%20Reference) (NormalImpulse :type Vector :default "0, 0, 0") (Hit :type Hit%20Result%20Structure%20%28by%20ref%29))
  (Game|QuitGame 0 "Quit" false))

(event EventBeginPlay
  (bind _returnvalue (UserInterface|CreateWidget "/Game/Character/EXP.EXP_C"))
  (bind _output_get (Variables|Default|SetExpWidget _returnvalue))
  (UserInterface|Viewport|AddtoViewport _output_get 0)
  (Default|Refresh (Variables|Default|GetExpWidget) (Variables|메인게임|GetExp) (Variables|메인게임|GetMaxExp)))

(event EventTick
  (params (DeltaSeconds :type Float%20%28single-precision%29))
  (bind _returnvalue (Transformation|GetActorLocation))
  (bind _outactors (Actor|GetAllActorsOfClass "/Game/Enemy/Enemy.Enemy_C"))
  (bind _returnvalue_2 (Class|GameplayStatics|GetActorArrayAverageLocation _outactors))
  (bind _returnvalue_3 (Game|SpawnActorfromClass "/Game/Character/Magic_Bullet.Magic_Bullet_C" (Math|Transform|MakeTransform _returnvalue (Math|Rotator|FindLookatRotation _returnvalue _returnvalue_2)) "Undefined" "MultiplyWithRoot" 0 0))
  (Variables|/Game/Character/Magic.Magic_C|SetDamage _returnvalue_3 2e+02))

(event Input|AxisEvents|InputAxisMoveForward
  (params (AxisValue :type Float%20%28single-precision%29))
  (움직임|MoveUp AxisValue))

(event Input|AxisEvents|InputAxisMoveRight
  (params (AxisValue :type Float%20%28single-precision%29))
  (움직임|MoveSide AxisValue))

(fn ConstructionScript)

(fn MoveUp
  (params (B :type Float%20%28double-precision%29))
  (bind _returnvalue (Transformation|GetActorLocation))
  (bind (_x _y _z) (Math|Vector|BreakVector _returnvalue))
  (Transformation|SetActorLocation (Math|Vector|MakeVector _x _y (Math|Interpolation|FInterpTo _z (+ (* (Variables|기본세팅|GetVelocity) B) _z) 0.05 5.0)) false false))

(fn MoveSide
  (params (B :type Float%20%28double-precision%29))
  (bind _returnvalue (Transformation|GetActorLocation))
  (bind (_x _y _z) (Math|Vector|BreakVector _returnvalue))
  (Transformation|SetActorLocation (Math|Vector|MakeVector (Math|Interpolation|FInterpTo _x (+ (* (Variables|기본세팅|GetVelocity) B) _x) 0.05 5.0) _y _z) false false))

(fn GetExp
  (params (Exp :type Float%20%28double-precision%29))
  (if (>= (+ Exp (Variables|메인게임|GetExp)) (Variables|메인게임|GetMaxExp))
    (Math|Integer|IncrementInt (Variables|메인게임|GetLevel)
      (:%20%20
        (Variables|메인게임|SetMaxExp (* (Variables|메인게임|GetMaxExp) 1.5))
        (Variables|메인게임|SetExp 0.0)))
    (else
      (Variables|메인게임|SetExp (+ Exp (Variables|메인게임|GetExp)))))
  (Default|Refresh (Variables|Default|GetExpWidget) (Variables|메인게임|GetExp) (Variables|메인게임|GetMaxExp)))